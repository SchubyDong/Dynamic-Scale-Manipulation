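; BP_Keyboard is an in-world numeric keypad that the scene's pen presses by overlapping key components to enter a two-digit Answer.
; Digit keys fill two slots in the KeyboardUI widget's text, where zero marks an empty slot.
; AC clears the display, and ENT stores the joined digits as Answer only when both are non-zero.
; Accepted presses beep, update press counters and share a half-second debounce.
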(event `self.ReceiveBeginPlay`
  (`self.AllClean_keyboardText`)
  (set `self.Is_NOT_Delaying` true)
  (set `self.KeyCounter` 0)
  (set `self.ACCounter` 0)
  (set `self.Answer` 0))

(event `self.ReceiveActorBeginOverlap`
  (params (OtherActor :type "Actor Object Reference")))

(event `self.0.OnComponentBeginOverlap`
  (params (OverlappedComponent :type "PrimitiveComponent Object Reference") (OtherActor :type "Actor Object Reference") (OtherComp :type "PrimitiveComponent Object Reference") (OtherBodyIndex :type Integer) (bFromSweep :type Boolean) (SweepResult :type "HitResult Structure (by ref)"))
  (if (and (== OtherActor (`self.Pen_In Scene`)) (`self.Is_NOT_Delaying`))
    (`self.Add_KeyboardText` 0)
    (`GameplayStatics.PlaySound2D` "/Game/Sound/S_Button_Beep.S_Button_Beep" 1.0 1.0 0.0 null null)
    (`/Engine/EditorBlueprintResources/StandardMacros.IncrementInt` (`self.KeyCounter`)
      (:`  `
        (set `self.Is_NOT_Delaying` false)
        (`KismetSystemLibrary.Delay` 0.5)
        (set `self.Is_NOT_Delaying` true)))))

(event `self.AC.OnComponentBeginOverlap`
  (params (OverlappedComponent :type "PrimitiveComponent Object Reference") (OtherActor :type "Actor Object Reference") (OtherComp :type "PrimitiveComponent Object Reference") (OtherBodyIndex :type Integer) (bFromSweep :type Boolean) (SweepResult :type "HitResult Structure (by ref)"))
  (if (and (== OtherActor (`self.Pen_In Scene`)) (`self.Is_NOT_Delaying`))
    (`self.AllClean_keyboardText`)
    (`GameplayStatics.PlaySound2D` "/Game/Sound/S_Button_Beep.S_Button_Beep" 1.0 1.0 0.0 null null)
    (`/Engine/EditorBlueprintResources/StandardMacros.IncrementInt` (`self.KeyCounter`)
      (:`  `
        (`/Engine/EditorBlueprintResources/StandardMacros.IncrementInt` (`self.ACCounter`)
          (:`  `
            (set `self.Is_NOT_Delaying` false)
            (`KismetSystemLibrary.Delay` 0.5)
            (set `self.Is_NOT_Delaying` true)))))))

(event `self.ENT.OnComponentBeginOverlap`
  (params (OverlappedComponent :type "PrimitiveComponent Object Reference") (OtherActor :type "Actor Object Reference") (OtherComp :type "PrimitiveComponent Object Reference") (OtherBodyIndex :type Integer) (bFromSweep :type Boolean) (SweepResult :type "HitResult Structure (by ref)"))
  (bind (_lefts _rights) (`KismetStringLibrary.Split` (`KismetTextLibrary.Conv_TextToString` (`TextBlock.GetText` (`/Game/VirtualRealityBP/Blueprints/Easiglow_Keyboard_UI.Value` (cast `/Game/VirtualRealityBP/Blueprints/Easiglow_Keyboard_UI` (`WidgetComponent.GetWidget` (`self.KeyboardUI`)) :!pure true)))) "    "))
  (if (and (== OtherActor (`self.Pen_In Scene`)) (`self.Is_NOT_Delaying`))
    (if (and (`KismetStringLibrary.NotEqual_StrStr` _lefts "0") (`KismetStringLibrary.NotEqual_StrStr` _rights "0"))
      (set `self.Answer` (`KismetStringLibrary.Conv_StringToInt` (`KismetStringLibrary.Concat_StrStr` _lefts _rights)))
      (`self.AllClean_keyboardText`)
      (`GameplayStatics.PlaySound2D` "/Game/Sound/S_Button_Beep.S_Button_Beep" 1.0 1.0 0.0 null null)
      (`/Engine/EditorBlueprintResources/StandardMacros.IncrementInt` (`self.KeyCounter`)
        (:`  `
          (set `self.Is_NOT_Delaying` false)
          (`KismetSystemLibrary.Delay` 0.5)
          (set `self.Is_NOT_Delaying` true))))))

(event `self.1.OnComponentBeginOverlap`
  (params (OverlappedComponent :type "PrimitiveComponent Object Reference") (OtherActor :type "Actor Object Reference") (OtherComp :type "PrimitiveComponent Object Reference") (OtherBodyIndex :type Integer) (bFromSweep :type Boolean) (SweepResult :type "HitResult Structure (by ref)"))
  (if (and (== OtherActor (`self.Pen_In Scene`)) (`self.Is_NOT_Delaying`))
    (`self.Add_KeyboardText` 1)
    (`GameplayStatics.PlaySound2D` "/Game/Sound/S_Button_Beep.S_Button_Beep" 1.0 1.0 0.0 null null)
    (`/Engine/EditorBlueprintResources/StandardMacros.IncrementInt` (`self.KeyCounter`)
      (:`  `
        (set `self.Is_NOT_Delaying` false)
        (`KismetSystemLibrary.Delay` 0.5)
        (set `self.Is_NOT_Delaying` true)))))

(event `self.2.OnComponentBeginOverlap`
  (params (OverlappedComponent :type "PrimitiveComponent Object Reference") (OtherActor :type "Actor Object Reference") (OtherComp :type "PrimitiveComponent Object Reference") (OtherBodyIndex :type Integer) (bFromSweep :type Boolean) (SweepResult :type "HitResult Structure (by ref)"))
  (if (and (== OtherActor (`self.Pen_In Scene`)) (`self.Is_NOT_Delaying`))
    (`self.Add_KeyboardText` 2)
    (`GameplayStatics.PlaySound2D` "/Game/Sound/S_Button_Beep.S_Button_Beep" 1.0 1.0 0.0 null null)
    (`/Engine/EditorBlueprintResources/StandardMacros.IncrementInt` (`self.KeyCounter`)
      (:`  `
        (set `self.Is_NOT_Delaying` false)
        (`KismetSystemLibrary.Delay` 0.5)
        (set `self.Is_NOT_Delaying` true)))))

(event `self.3.OnComponentBeginOverlap`
  (params (OverlappedComponent :type "PrimitiveComponent Object Reference") (OtherActor :type "Actor Object Reference") (OtherComp :type "PrimitiveComponent Object Reference") (OtherBodyIndex :type Integer) (bFromSweep :type Boolean) (SweepResult :type "HitResult Structure (by ref)"))
  (if (and (== OtherActor (`self.Pen_In Scene`)) (`self.Is_NOT_Delaying`))
    (`self.Add_KeyboardText` 3)
    (`GameplayStatics.PlaySound2D` "/Game/Sound/S_Button_Beep.S_Button_Beep" 1.0 1.0 0.0 null null)
    (`/Engine/EditorBlueprintResources/StandardMacros.IncrementInt` (`self.KeyCounter`)
      (:`  `
        (set `self.Is_NOT_Delaying` false)
        (`KismetSystemLibrary.Delay` 0.5)
        (set `self.Is_NOT_Delaying` true)))))

(event `self.4.OnComponentBeginOverlap`
  (params (OverlappedComponent :type "PrimitiveComponent Object Reference") (OtherActor :type "Actor Object Reference") (OtherComp :type "PrimitiveComponent Object Reference") (OtherBodyIndex :type Integer) (bFromSweep :type Boolean) (SweepResult :type "HitResult Structure (by ref)"))
  (if (and (== OtherActor (`self.Pen_In Scene`)) (`self.Is_NOT_Delaying`))
    (`self.Add_KeyboardText` 4)
    (`GameplayStatics.PlaySound2D` "/Game/Sound/S_Button_Beep.S_Button_Beep" 1.0 1.0 0.0 null null)
    (`/Engine/EditorBlueprintResources/StandardMacros.IncrementInt` (`self.KeyCounter`)
      (:`  `
        (set `self.Is_NOT_Delaying` false)
        (`KismetSystemLibrary.Delay` 0.5)
        (set `self.Is_NOT_Delaying` true)))))

(event `self.5.OnComponentBeginOverlap`
  (params (OverlappedComponent :type "PrimitiveComponent Object Reference") (OtherActor :type "Actor Object Reference") (OtherComp :type "PrimitiveComponent Object Reference") (OtherBodyIndex :type Integer) (bFromSweep :type Boolean) (SweepResult :type "HitResult Structure (by ref)"))
  (if (and (== OtherActor (`self.Pen_In Scene`)) (`self.Is_NOT_Delaying`))
    (`self.Add_KeyboardText` 5)
    (`GameplayStatics.PlaySound2D` "/Game/Sound/S_Button_Beep.S_Button_Beep" 1.0 1.0 0.0 null null)
    (`/Engine/EditorBlueprintResources/StandardMacros.IncrementInt` (`self.KeyCounter`)
      (:`  `
        (set `self.Is_NOT_Delaying` false)
        (`KismetSystemLibrary.Delay` 0.5)
        (set `self.Is_NOT_Delaying` true)))))

(event `self.6.OnComponentBeginOverlap`
  (params (OverlappedComponent :type "PrimitiveComponent Object Reference") (OtherActor :type "Actor Object Reference") (OtherComp :type "PrimitiveComponent Object Reference") (OtherBodyIndex :type Integer) (bFromSweep :type Boolean) (SweepResult :type "HitResult Structure (by ref)"))
  (if (and (== OtherActor (`self.Pen_In Scene`)) (`self.Is_NOT_Delaying`))
    (`self.Add_KeyboardText` 6)
    (`GameplayStatics.PlaySound2D` "/Game/Sound/S_Button_Beep.S_Button_Beep" 1.0 1.0 0.0 null null)
    (`/Engine/EditorBlueprintResources/StandardMacros.IncrementInt` (`self.KeyCounter`)
      (:`  `
        (set `self.Is_NOT_Delaying` false)
        (`KismetSystemLibrary.Delay` 0.5)
        (set `self.Is_NOT_Delaying` true)))))

(event `self.8.OnComponentBeginOverlap`
  (params (OverlappedComponent :type "PrimitiveComponent Object Reference") (OtherActor :type "Actor Object Reference") (OtherComp :type "PrimitiveComponent Object Reference") (OtherBodyIndex :type Integer) (bFromSweep :type Boolean) (SweepResult :type "HitResult Structure (by ref)"))
  (if (and (== OtherActor (`self.Pen_In Scene`)) (`self.Is_NOT_Delaying`))
    (`self.Add_KeyboardText` 8)
    (`GameplayStatics.PlaySound2D` "/Game/Sound/S_Button_Beep.S_Button_Beep" 1.0 1.0 0.0 null null)
    (`/Engine/EditorBlueprintResources/StandardMacros.IncrementInt` (`self.KeyCounter`)
      (:`  `
        (set `self.Is_NOT_Delaying` false)
        (`KismetSystemLibrary.Delay` 0.5)
        (set `self.Is_NOT_Delaying` true)))))

(event `self.7.OnComponentBeginOverlap`
  (params (OverlappedComponent :type "PrimitiveComponent Object Reference") (OtherActor :type "Actor Object Reference") (OtherComp :type "PrimitiveComponent Object Reference") (OtherBodyIndex :type Integer) (bFromSweep :type Boolean) (SweepResult :type "HitResult Structure (by ref)"))
  (if (and (== OtherActor (`self.Pen_In Scene`)) (`self.Is_NOT_Delaying`))
    (`self.Add_KeyboardText` 7)
    (`GameplayStatics.PlaySound2D` "/Game/Sound/S_Button_Beep.S_Button_Beep" 1.0 1.0 0.0 null null)
    (`/Engine/EditorBlueprintResources/StandardMacros.IncrementInt` (`self.KeyCounter`)
      (:`  `
        (set `self.Is_NOT_Delaying` false)
        (`KismetSystemLibrary.Delay` 0.5)
        (set `self.Is_NOT_Delaying` true)))))

(event `self.9.OnComponentBeginOverlap`
  (params (OverlappedComponent :type "PrimitiveComponent Object Reference") (OtherActor :type "Actor Object Reference") (OtherComp :type "PrimitiveComponent Object Reference") (OtherBodyIndex :type Integer) (bFromSweep :type Boolean) (SweepResult :type "HitResult Structure (by ref)"))
  (if (and (== OtherActor (`self.Pen_In Scene`)) (`self.Is_NOT_Delaying`))
    (`self.Add_KeyboardText` 9)
    (`GameplayStatics.PlaySound2D` "/Game/Sound/S_Button_Beep.S_Button_Beep" 1.0 1.0 0.0 null null)
    (`/Engine/EditorBlueprintResources/StandardMacros.IncrementInt` (`self.KeyCounter`)
      (:`  `
        (set `self.Is_NOT_Delaying` false)
        (`KismetSystemLibrary.Delay` 0.5)
        (set `self.Is_NOT_Delaying` true)))))

(fn `Add_KeyboardText`
  (params (Number :type Integer))
  (bind _returnvalue (`KismetStringLibrary.Conv_IntToString` Number))
  (bind _value (`/Game/VirtualRealityBP/Blueprints/Easiglow_Keyboard_UI.Value` (cast `/Game/VirtualRealityBP/Blueprints/Easiglow_Keyboard_UI` (`WidgetComponent.GetWidget` (`self.KeyboardUI`)) :!pure true)))
  (bind (_lefts _rights) (`KismetStringLibrary.Split` (`KismetTextLibrary.Conv_TextToString` (`TextBlock.GetText` _value)) "    "))
  (if (== (`KismetStringLibrary.Conv_StringToInt` _lefts) 0)
    (`TextBlock.SetText` _value (`KismetTextLibrary.Conv_StringToText` (`KismetStringLibrary.Concat_StrStr` _returnvalue "    " "0")))
    (elif (== (`KismetStringLibrary.Conv_StringToInt` _rights) 0)
      (`TextBlock.SetText` _value (`KismetTextLibrary.Conv_StringToText` (`KismetStringLibrary.Concat_StrStr` _lefts "    " _returnvalue))))))

(fn `AllClean_keyboardText`
  (`TextBlock.SetText` (`/Game/VirtualRealityBP/Blueprints/Easiglow_Keyboard_UI.Value` (cast `/Game/VirtualRealityBP/Blueprints/Easiglow_Keyboard_UI` (`WidgetComponent.GetWidget` (`self.KeyboardUI`)) :!pure true)) "0    0"))

(fn `UserConstructionScript`)